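; BP_3Dto2D is a work-in-progress skill that turns the third-person character into a flat 2D form.
; Sphere overlap caches the character and triggers flattening: zero Z mesh scale, disabled movement, camera shift.
; Tick traces at a fixed world offset, snapping the character to hits and flattening it.
; The camera shift moves the camera's owner to origin, rotated by the hit normal; skill events are stubs and ManaCheck is uncalled.
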(event OnComponentBeginOverlap(Sphere)
  (params (OverlappedComponent :type Primitive%20Component%20Object%20Reference) (OtherActor :type Actor%20Object%20Reference) (OtherComp :type Primitive%20Component%20Object%20Reference) (OtherBodyIndex :type Integer) (bFromSweep :type Boolean) (SweepResult :type Hit%20Result%20Structure%20%28by%20ref%29))
  (bind _asbp_third_person_character (Utilities|Casting|CastToBP_ThirdPersonCharacter OtherActor))
  (Variables|Default|SetAs%20BP%20Third%20Person%20Character _asbp_third_person_character)
  (CallFunction|ActivateFlatForm))

(event Custom|ActivateFlatForm
  (CallFunction|ShiftCamerato2D)
  (Transformation|SetRelativeScale3D (Variables|/Script/Engine.Character|GetMesh (Variables|Default|GetAs%20BP%20Third%20Person%20Character)) "1.000000,1.000000,0.000000")
  (Pawn|Components|CharacterMovement|DisableMovement (Variables|/Script/Engine.Character|GetCharacterMovement (Variables|Default|GetAs%20BP%20Third%20Person%20Character))))

(event Custom|ShiftCamerato2D
  (Development|PrintString "camera changing")
  (Transformation|SetActorLocation (Components|GetOwner (Variables|/Game/ThirdPerson/Blueprints/BP_ThirdPersonCharacter.BP_ThirdPersonCharacter_C|GetFirstPersonCamera (Variables|Default|GetAs%20BP%20Third%20Person%20Character))) "0, 0, 0" false false)
  (Transformation|SetActorRotation (Components|GetOwner (Variables|/Game/ThirdPerson/Blueprints/BP_ThirdPersonCharacter.BP_ThirdPersonCharacter_C|GetFirstPersonCamera (Variables|Default|GetAs%20BP%20Third%20Person%20Character))) (Math|Rotator|MakeRotfromZ (.Normal (Collision|BreakHitResult (stale EventTick _outhit))))))

(event EventHoldSkill)

(event EventEndSkill)

(event EventTick
  (params (DeltaSeconds :type Float%20%28single-precision%29))
  (bind _as_bp_third_person_character (Variables|Default|GetAs%20BP%20Third%20Person%20Character))
  (bind _returnvalue (Transformation|GetActorLocation _as_bp_third_person_character))
  (bind _outhit (Collision|LineTraceByChannel _returnvalue (+ _returnvalue (+ (Math|Conversions|ToVector(Float) 2e+02) (Math|Vector|MakeVector 0.0 0.0 -1e+02))) "TraceTypeQuery1" false 0 "ForDuration"))
  (if (.bBlockingHit (Collision|BreakHitResult _outhit))
    (Transformation|SetActorLocation (Variables|Default|GetAs%20BP%20Third%20Person%20Character) (+ (.ImpactPoint (Collision|BreakHitResult _outhit)) "0.000000,0.000000,100.000000") false false)
    (CallFunction|ActivateFlatForm)))

(event EventBeginSkill)

(fn ConstructionScript)

(fn ActivateFlatForm)

(fn ShiftCamerato2D)